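; Door actor that shows an unlock or open prompt and advances the story when its StageUnlocked event runs.
; A looping timer clears the prompt once the player is out of range.
; StageUnlocked branches on numbered actor tags and player Stage to update thoughts, cellmate dialogue and HUD missions.
; The tag 7 branch also stages the cellmate and guard deaths by swapping flipbooks.
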(event EventBeginPlay
  (bind _returnvalue (UserInterface|CreateWidget "/Game/Widgets/W_Enemy.W_Enemy_C"))
  (UserInterface|SetWidget (Variables|Default|GetText) _returnvalue)
  (Utilities|Time|SetTimerbyFunctionName 0 "ResetText" 1.0 true)
  (bind _asbp_player (Utilities|Casting|CastToBP_Player (Game|Player|GetPlayerPawn 0)))
  (Utilities|FlowControl|Delay 2.0)
  (Variables|Default|SetToughts (Variables|/Game/Blueprints/BP_Player.BP_Player_C|GetToughts _asbp_player))
  (Variables|Default|SetHUD (Variables|/Game/Blueprints/BP_Player.BP_Player_C|GetHUD _asbp_player))
  (bind _returnvalue_2 (Actor|GetActorOfClass "/Game/Blueprints/BP_CellMate.BP_CellMate_C"))
  (bind _asw_enemy (Utilities|Casting|CastToW_Enemy (UserInterface|GetUserWidgetObject (Variables|/Game/Blueprints/BP_CellMate.BP_CellMate_C|GetText _returnvalue_2)))))

(event Collision|EventActorBeginOverlap
  (params (OtherActor :type Actor%20Object%20Reference)))

(event EventTick
  (params (DeltaSeconds :type Float%20%28single-precision%29)))

(event EventShowOptions
  (bind _asw_enemy (Utilities|Casting|CastToW_Enemy (UserInterface|GetUserWidgetObject (Variables|Default|GetText))))
  (if (Variables|Default|GetLocked)
    (Rendering|Components|TextRender|SetText (Variables|/Game/Widgets/W_Enemy.W_Enemy_C|GetEnemyText _asw_enemy) "(U) Unlock")
    (else
      (Rendering|Components|TextRender|SetText (Variables|/Game/Widgets/W_Enemy.W_Enemy_C|GetEnemyText _asw_enemy) "(O) Open"))))

(event EventStageUnlocked
  (bind _tags (Variables|Actor|GetTags))
  (bind _hud (Variables|Default|GetHUD))
  (bind _hud_2 (Variables|Default|GetHUD))
  (bind _missiontext (Variables|/Game/Widgets/WB_HUD.WB_HUD_C|GetMissionText _hud))
  (bind _missiontext_2 (Variables|/Game/Widgets/WB_HUD.WB_HUD_C|GetMissionText _hud_2))
  (if (and (Utilities|Array|ContainsItem _tags "1") (< (Variables|/Game/Blueprints/BP_Player.BP_Player_C|GetStage (stale EventBeginPlay _asbp_player)) 1))
    (Variables|/Game/Blueprints/BP_Player.BP_Player_C|SetStage (stale EventBeginPlay _asbp_player) 1)
    (Rendering|Components|TextRender|SetText (Variables|/Game/Widgets/W_Toughts.W_Toughts_C|GetText (Variables|/Game/Blueprints/BP_Player.BP_Player_C|GetToughts (stale EventBeginPlay _asbp_player))) "...that was easy...")
    (Utilities|FlowControl|Delay 0.5)
    (Default|ShowSelf (Variables|/Game/Blueprints/BP_Player.BP_Player_C|GetToughts (stale EventBeginPlay _asbp_player)))
    (Rendering|Components|TextRender|SetText (Variables|/Game/Widgets/W_Enemy.W_Enemy_C|GetEnemyText (stale EventBeginPlay _asw_enemy)) "BUDDY 
Well done, mate!")
    (Rendering|Components|TextRender|SetText _missiontext "Feed the inmates")
    (Utilities|FlowControl|Delay 2.0)
    (Rendering|Components|TextRender|SetText (Variables|/Game/Widgets/W_Enemy.W_Enemy_C|GetEnemyText (stale EventBeginPlay _asw_enemy)) "BUDDY")
    (elif (and (Utilities|Array|ContainsItem _tags "2") (< (Variables|/Game/Blueprints/BP_Player.BP_Player_C|GetStage (stale EventBeginPlay _asbp_player)) 2))
      (Variables|/Game/Blueprints/BP_Player.BP_Player_C|SetStage (stale EventBeginPlay _asbp_player) 2)
      (Rendering|Components|TextRender|SetText (Variables|/Game/Widgets/W_Toughts.W_Toughts_C|GetText (Variables|/Game/Blueprints/BP_Player.BP_Player_C|GetToughts (stale EventBeginPlay _asbp_player))) "...helping them felt...good!")
      (Utilities|FlowControl|Delay 0.5)
      (Default|ShowSelf (Variables|/Game/Blueprints/BP_Player.BP_Player_C|GetToughts (stale EventBeginPlay _asbp_player)))
      (Rendering|Components|TextRender|SetText (Variables|/Game/Widgets/W_Enemy.W_Enemy_C|GetEnemyText (stale EventBeginPlay _asw_enemy)) "BUDDY 
That was nice of you!")
      (Rendering|Components|TextRender|SetText _missiontext "")
      (Utilities|FlowControl|Delay 2.0)
      (Rendering|Components|TextRender|SetText (Variables|/Game/Widgets/W_Enemy.W_Enemy_C|GetEnemyText (stale EventBeginPlay _asw_enemy)) "BUDDY")
      (elif (and (Utilities|Array|ContainsItem _tags "4") (< (Variables|/Game/Blueprints/BP_Player.BP_Player_C|GetStage (stale EventBeginPlay _asbp_player)) 4))
        (Rendering|Components|TextRender|SetText (Variables|/Game/Widgets/W_Enemy.W_Enemy_C|GetEnemyText (stale EventBeginPlay _asw_enemy)) "BUDDY 
I'm glad we're in this together, bud!")
        (Rendering|Components|TextRender|SetText _missiontext "Follow the path")
        (Utilities|FlowControl|Delay 4.0)
        (Rendering|Components|TextRender|SetText (Variables|/Game/Widgets/W_Toughts.W_Toughts_C|GetText (Variables|/Game/Blueprints/BP_Player.BP_Player_C|GetToughts (stale EventBeginPlay _asbp_player))) "...it IS nice to have a friend")
        (Default|ShowSelf (Variables|/Game/Blueprints/BP_Player.BP_Player_C|GetToughts (stale EventBeginPlay _asbp_player)))
        (Rendering|Components|TextRender|SetText (Variables|/Game/Widgets/W_Enemy.W_Enemy_C|GetEnemyText (stale EventBeginPlay _asw_enemy)) "BUDDY")
        (elif (Utilities|Array|ContainsItem _tags "7")
          (if (< (Variables|/Game/Blueprints/BP_Player.BP_Player_C|GetStage (stale EventBeginPlay _asbp_player)) 7)
            (Variables|/Game/Blueprints/BP_Player.BP_Player_C|SetStage (stale EventBeginPlay _asbp_player) 7)
            (Sprite|SetFlipbook (Variables|/Game/Blueprints/BP_CellMate.BP_CellMate_C|GetPaperFlipbook (stale EventBeginPlay _returnvalue_2)) "/Game/Assets/Player/Death/FB_NPCDead.FB_NPCDead")
            (Transformation|SetActorLocation (stale EventBeginPlay _returnvalue_2) (- (Transformation|GetActorLocation (stale EventBeginPlay _returnvalue_2)) "-60.000000,0.000000,0.000000") false false)
            (bind _returnvalue (Actor|GetActorOfClass "/Game/Blueprints/BP_Guard.BP_Guard_C"))
            (Variables|/Game/Blueprints/BP_Guard.BP_Guard_C|SetDead _returnvalue true)
            (Sprite|SetFlipbook (Variables|/Game/Blueprints/BP_Guard.BP_Guard_C|GetPaperFlipbook _returnvalue) "/Game/Assets/NPC/Guard/Death/FB_GuardDead.FB_GuardDead")
            (bind _asw_enemy (Utilities|Casting|CastToW_Enemy (UserInterface|GetWidget (Variables|/Game/Blueprints/BP_Guard.BP_Guard_C|GetText _returnvalue))))
            (Rendering|Components|TextRender|SetText (Variables|/Game/Widgets/W_Enemy.W_Enemy_C|GetEnemyText _asw_enemy) "")
            (Rendering|Components|TextRender|SetText (Variables|/Game/Widgets/W_Enemy.W_Enemy_C|GetEnemyText (stale EventBeginPlay _asw_enemy)) "")
            (Rendering|Components|TextRender|SetText (Variables|/Game/Widgets/W_Toughts.W_Toughts_C|GetText (Variables|/Game/Blueprints/BP_Player.BP_Player_C|GetToughts (stale EventBeginPlay _asbp_player))) "...silence?...wait, does this mean....BUDDY?")
            (Utilities|FlowControl|Delay 2.0)
            (Default|ShowSelf (Variables|/Game/Blueprints/BP_Player.BP_Player_C|GetToughts (stale EventBeginPlay _asbp_player)))
            (elif (== (Variables|/Game/Blueprints/BP_Player.BP_Player_C|GetStage (stale EventBeginPlay _asbp_player)) 7)
              (Variables|/Game/Blueprints/BP_Player.BP_Player_C|SetStage (stale EventBeginPlay _asbp_player) 8)
              (Utilities|FlowControl|Delay 2.0)
              (Rendering|Components|TextRender|SetText (Variables|/Game/Widgets/W_Toughts.W_Toughts_C|GetText (Variables|/Game/Blueprints/BP_Player.BP_Player_C|GetToughts (stale EventBeginPlay _asbp_player))) "...no...NO...I shouldn't have left you...I'm so sorry...")
              (Default|ShowSelf (Variables|/Game/Blueprints/BP_Player.BP_Player_C|GetToughts (stale EventBeginPlay _asbp_player)))))
          (elif (and (Utilities|Array|ContainsItem _tags "8") (or (== (Variables|/Game/Blueprints/BP_Player.BP_Player_C|GetStage (stale EventBeginPlay _asbp_player)) 7) (== (Variables|/Game/Blueprints/BP_Player.BP_Player_C|GetStage (stale EventBeginPlay _asbp_player)) 8)))
            (Rendering|Components|TextRender|SetText _missiontext_2 "Help or kill him!")
            (elif (Utilities|Array|ContainsItem _tags "9")
              (Variables|/Game/Blueprints/BP_Player.BP_Player_C|SetStage (stale EventBeginPlay _asbp_player) 9)
              (Rendering|Components|TextRender|SetText _missiontext_2 "")
              (elif (Utilities|Array|ContainsItem _tags "10")
                (Rendering|Components|TextRender|SetText _missiontext_2 "You know what to do")))))))))

(fn ConstructionScript)

(fn ResetText
  (bind _asw_enemy (Utilities|Casting|CastToW_Enemy (UserInterface|GetUserWidgetObject (Variables|Default|GetText))))
  (if (>= (Transformation|GetDistanceTo (Game|Player|GetPlayerPawn 0)) 9e+01)
    (Rendering|Components|TextRender|SetText (Variables|/Game/Widgets/W_Enemy.W_Enemy_C|GetEnemyText _asw_enemy) "")))