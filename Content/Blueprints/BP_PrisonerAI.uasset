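; AI controller for a hungry 2D prisoner NPC, driving speech text, aggression and death.
; Pawn tags choose dialogue and behaviour: violent prisoners threaten an overlapping player, chase without pathfinding, sphere-trace melee hits, and return to start when outdistanced.
; Tick branches on Health and Hunger: fed prisoners show thanks, while dead ones swap flipbook and, unless tagged lead2, give the player a key.
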(event EventBeginPlay
  (bind _returnvalue (Pawn|GetControlledPawn))
  (bind _tags (Variables|/Script/Engine.Actor|GetTags _returnvalue))
  (bind _asbp_prisoner (Utilities|Casting|CastToBP_Prisoner _returnvalue))
  (Utilities|FlowControl|Delay 1.0)
  (bind _asw_enemy (Utilities|Casting|CastToW_Enemy (UserInterface|GetUserWidgetObject (Variables|/Game/Blueprints/BP_Prisoner.BP_Prisoner_C|GetText _asbp_prisoner))))
  (if (Utilities|Array|ContainsItem _tags "lead1")
    (Rendering|Components|TextRender|SetText (Variables|/Game/Widgets/W_Enemy.W_Enemy_C|GetEnemyText _asw_enemy) "Ther' ain' no food fo' all o' us!!!")
    (Variables|/Game/Blueprints/BP_Prisoner.BP_Prisoner_C|SetTextLength _asbp_prisoner (Utilities|String|Len (Utilities|String|ToString(Text) (Class|TextBlock|GetText (Variables|/Game/Widgets/W_Enemy.W_Enemy_C|GetEnemyText _asw_enemy)))) :!label _label)
    (elif (Utilities|Array|ContainsItem _tags "lead2")
      (Rendering|Components|TextRender|SetText (Variables|/Game/Widgets/W_Enemy.W_Enemy_C|GetEnemyText _asw_enemy) "YOU'RE GOIN' DOWN, Y'ALL!")
      (goto _label))))

(event EventTick
  (params (DeltaSeconds :type Float%20%28single-precision%29))
  (bind _returnvalue (Game|Player|GetPlayerPawn 0))
  (bind _returnvalue_2 (Pawn|GetControlledPawn))
  (bind _returnvalue_3 (Transformation|GetActorLocation _returnvalue))
  (bind _tags (Variables|/Script/Engine.Actor|GetTags _returnvalue_2))
  (bind _returnvalue_4 (Utilities|Array|ContainsItem _tags "lead2"))
  (if (> (Variables|/Game/Blueprints/BP_Prisoner.BP_Prisoner_C|GetHealth (stale EventBeginPlay _asbp_prisoner)) 0.0)
    (if (>= (Variables|/Game/Blueprints/BP_Prisoner.BP_Prisoner_C|GetHunger (stale EventBeginPlay _asbp_prisoner)) 0)
      (if (Utilities|Array|ContainsItem _tags "violent")
        (if (Variables|/Game/Blueprints/BP_Prisoner.BP_Prisoner_C|GetAttacking (stale EventBeginPlay _asbp_prisoner))
          (if (and (> (Variables|/Game/Blueprints/BP_Prisoner.BP_Prisoner_C|GetHealth (stale EventBeginPlay _asbp_prisoner)) 0.0) (>= (Variables|/Game/Blueprints/BP_Prisoner.BP_Prisoner_C|GetHunger (stale EventBeginPlay _asbp_prisoner)) 0))
            (if (not (Variables|/Game/Blueprints/BP_Prisoner.BP_Prisoner_C|GetStopped (stale EventBeginPlay _asbp_prisoner)))
              (AI|Navigation|MovetoLocation _returnvalue_3 0.0 false false false true 0)
              (if (> (Variables|/Game/Blueprints/BP_Prisoner.BP_Prisoner_C|GetHealth (stale EventBeginPlay _asbp_prisoner)) 0.0)
                (switch int (Math|Float|Truncate (Math|Float|Sign(Float) (.z (- _returnvalue_3 (Transformation|GetActorLocation (stale EventBeginPlay _asbp_prisoner))))))
                  (:Default
                    _)
                  (:-1
                    (Sprite|SetFlipbook (Variables|/Game/Blueprints/BP_Prisoner.BP_Prisoner_C|GetPaperFlipbook (stale EventBeginPlay _asbp_prisoner)) "/Game/Assets/Player/WalkDown/FB_WalkDown.FB_WalkDown"))
                  (:0
                    _)
                  (:1
                    (Sprite|SetFlipbook (Variables|/Game/Blueprints/BP_Prisoner.BP_Prisoner_C|GetPaperFlipbook (stale EventBeginPlay _asbp_prisoner)) "/Game/Assets/Player/WalkUp/FB_WalkUp.FB_WalkUp")))
                (if (<= (Transformation|GetDistanceTo (stale EventBeginPlay _asbp_prisoner) _returnvalue) 2e+01)
                  (AI|Navigation|StopMovement)
                  (Variables|/Game/Blueprints/BP_Prisoner.BP_Prisoner_C|SetStopped (stale EventBeginPlay _asbp_prisoner) true)
                  (Utilities|FlowControl|Delay 0.5)
                  (if (> (Variables|/Game/Blueprints/BP_Prisoner.BP_Prisoner_C|GetHealth (stale EventBeginPlay _asbp_prisoner)) 0.0)
                    (bind _outhit (Collision|SphereTraceByChannel (Transformation|GetActorLocation (stale EventBeginPlay _asbp_prisoner)) (+ (Transformation|GetActorLocation (stale EventBeginPlay _asbp_prisoner)) (Math|Vector|MakeVector (* (Class|KismetMathLibrary|SignOfInteger64 (.ReturnValue (Class|KismetMathLibrary|FMod64 (.x (- _returnvalue_3 (Transformation|GetActorLocation (stale EventBeginPlay _asbp_prisoner)))) 1e+01))) 1e+01) 0.0 (* (Class|KismetMathLibrary|SignOfInteger64 (.ReturnValue (Class|KismetMathLibrary|FMod64 (.z (- _returnvalue_3 (Transformation|GetActorLocation (stale EventBeginPlay _asbp_prisoner)))) 1e+01))) 1e+01))) 1e+01 "TraceTypeQuery4" false 0 "None"))
                    (Variables|/Game/Blueprints/BP_Prisoner.BP_Prisoner_C|SetStopped (stale EventBeginPlay _asbp_prisoner) false)
                    (bind _asbp_player (Utilities|Casting|CastToBP_Player (.hitactor _outhit)))
                    (Game|Damage|ApplyDamage _asbp_player 1e+01 0 0)
                    (Audio|PlaySound2D "/Game/Assets/Sound/man_hurt3.man_hurt3" 1.0 1.0 0.0 0 0))
                  (elif (>= (Transformation|GetDistanceTo (stale EventBeginPlay _asbp_prisoner) _returnvalue) 1e+02)
                    (Variables|/Game/Blueprints/BP_Prisoner.BP_Prisoner_C|SetAttacking (stale EventBeginPlay _asbp_prisoner) false)
                    (AI|Navigation|MovetoLocation (Variables|/Game/Blueprints/BP_Prisoner.BP_Prisoner_C|GetStartPoint (stale EventBeginPlay _asbp_prisoner)) 0.0 true false false true 0 false))))))
          (else
            (bind _playerclose (CallFunction|CheckActorClose (stale EventBeginPlay _asbp_prisoner)))
            (if _playerclose
              (Rendering|Components|TextRender|SetText (Variables|/Game/Widgets/W_Enemy.W_Enemy_C|GetEnemyText (stale EventBeginPlay _asw_enemy)) "Gimme somethin' to eat unless you wanna be the food!")
              (Variables|/Game/Blueprints/BP_Prisoner.BP_Prisoner_C|SetTextLength (stale EventBeginPlay _asbp_prisoner) (Utilities|String|Len (Utilities|String|ToString(Text) (Class|TextBlock|GetText (Variables|/Game/Widgets/W_Enemy.W_Enemy_C|GetEnemyText (stale EventBeginPlay _asw_enemy))))))
              (Utilities|FlowControl|Delay 2.0)
              (Variables|/Game/Blueprints/BP_Prisoner.BP_Prisoner_C|SetAttacking (stale EventBeginPlay _asbp_prisoner) true)
              (Rendering|Components|TextRender|SetText (Variables|/Game/Widgets/W_Enemy.W_Enemy_C|GetEnemyText (stale EventBeginPlay _asw_enemy)) "FOOOD!!")
              (Variables|/Game/Blueprints/BP_Prisoner.BP_Prisoner_C|SetTextLength (stale EventBeginPlay _asbp_prisoner) (Utilities|String|Len (Utilities|String|ToString(Text) (Class|TextBlock|GetText (Variables|/Game/Widgets/W_Enemy.W_Enemy_C|GetEnemyText (stale EventBeginPlay _asw_enemy))))))))))
      (else
        (if _returnvalue_4
          (Rendering|Components|TextRender|SetText (Variables|/Game/Widgets/W_Enemy.W_Enemy_C|GetEnemyText (stale EventBeginPlay _asw_enemy)) "Thank' mate, I was so hungry I could'a killed s'm'one!")
          (else
            (Rendering|Components|TextRender|SetText (Variables|/Game/Widgets/W_Enemy.W_Enemy_C|GetEnemyText (stale EventBeginPlay _asw_enemy)) "Ya've saved m'life, mate! I'll give yah this key.")))
        (Variables|/Game/Blueprints/BP_Prisoner.BP_Prisoner_C|SetTextLength (stale EventBeginPlay _asbp_prisoner) (Utilities|String|Len (Utilities|String|ToString(Text) (Class|TextBlock|GetText (Variables|/Game/Widgets/W_Enemy.W_Enemy_C|GetEnemyText (stale EventBeginPlay _asw_enemy))))))
        (Utilities|FlowControl|Delay 1e+01)
        (Variables|/Game/Blueprints/BP_Prisoner.BP_Prisoner_C|SetTextLength (stale EventBeginPlay _asbp_prisoner) 0)))
    (else
      (Rendering|Components|TextRender|SetText (Variables|/Game/Widgets/W_Enemy.W_Enemy_C|GetEnemyText (stale EventBeginPlay _asw_enemy)) "")
      (Sprite|SetFlipbook (Variables|/Game/Blueprints/BP_Prisoner.BP_Prisoner_C|GetPaperFlipbook (stale EventBeginPlay _asbp_prisoner)) "/Game/Assets/Player/Death/FB_NPCDead.FB_NPCDead")
      (if (not _returnvalue_4)
        (Audio|PlaySoundatLocation "/Game/Assets/Sound/key-get-39925.key-get-39925" (Transformation|GetActorLocation (Game|Player|GetPlayerPawn 0)) "0, 0, 0" 1.0 1.0 0.0 0 0 0 0)
        (bind _asbp_player_2 (Utilities|Casting|CastToBP_Player (Game|Player|GetPlayerPawn 0)))
        (Variables|/Game/Blueprints/BP_Player.BP_Player_C|SetHasKey _asbp_player_2 true)))))

(fn ConstructionScript)

(fn CheckActorClose
  (params (Actor :type BP%20Prisoner%20Object%20Reference))
  (return (Collision|IsOverlappingActor Actor (Game|Player|GetPlayerPawn 0) :!class /Script/Engine.Actor)))