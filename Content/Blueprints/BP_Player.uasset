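; Paper2D player pawn for a prison escape game, with directional flipbook movement, punching, health and draining hunger that damages at zero.
; Forward sphere traces along the last move direction drive option prompts and key actions: looting food, eating rats, feeding prisoners for keys, and unlocking or passing doors.
; Punches damage rats, prisoners and a guard inline.
; Kills trigger thought-widget lines, or a scripted fade-out ending for the guard; death opens a menu.
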(event Custom|Increase%20Hunger
  (params (Amount :type Float%20%28double-precision%29))
  ;[0.15 0.15 0.15 0.5] Increase hunger
  (Variables|Default|SetHunger (+ (Variables|Default|GetHunger) Amount))
  (if (> (Variables|Default|GetHunger) 1e+02)
    (Variables|Default|SetHunger 1e+02)))

(event Custom|Decrease%20Hunger
  (params (Amount :type Float%20%28double-precision%29))
  ;[0.15 0.15 0.15 0.5] Decrease hunger and apply damage if hunger=0
  (Variables|Default|SetHunger (- (Variables|Default|GetHunger) Amount))
  (if (< (Variables|Default|GetHunger) 0.0)
    (Variables|Default|SetHunger 0.0)
    (Game|Damage|ApplyDamage self (* (stale EventTick DeltaSeconds) 2.0) 0 0)))

(event Input|EnhancedActionEvents|EnhancedInputActionIA_Pause
  (params (ActionValue :type Boolean) (ElapsedSeconds :type Float%20%28double-precision%29) (TriggeredSeconds :type Float%20%28double-precision%29) (InputAction :type Input%20Action%20Object%20Reference :default "/Game/Input/IA_Pause.IA_Pause"))
  (bind _returnvalue (Game|GetPlayerController 0))
  ;[0.15 0.15 0.15 0.5] Open pause menu when "esc" pressed
  (:Started
    (bind _returnvalue_2 (UserInterface|CreateWidget "/Game/Widgets/WB_PauseMenu.WB_PauseMenu_C"))
    (UserInterface|Viewport|AddtoViewport _returnvalue_2 0)
    (Variables|/Script/Engine.PlayerController|SetbShowMouseCursor _returnvalue true)
    (Input|SetInputModeUIOnly _returnvalue 0 "DoNotLock" false)
    (Game|SetGamePaused true)))

(event Input|EnhancedActionEvents|EnhancedInputActionIA_Move
  (params (ActionValue :type Vector%202D%20Structure) (ElapsedSeconds :type Float%20%28double-precision%29) (TriggeredSeconds :type Float%20%28double-precision%29) (InputAction :type Input%20Action%20Object%20Reference :default "/Game/Input/IA_Move.IA_Move"))
  (Pawn|Input|AddMovementInput (Transformation|GetActorUpVector) (.x ActionValue) false)
  (Pawn|Input|AddMovementInput (Transformation|GetActorForwardVector) (.y ActionValue) false)
  (bind _output_get (Variables|Default|SetDirection (Math|Vector|MakeVector (Math|Float|Sign(Float) (.y ActionValue)) 0.0 (Math|Float|Sign(Float) (.x ActionValue)))))
  (switch int (Math|Float|Truncate (.z _output_get))
    (:-1
      (Sprite|SetFlipbook (Variables|Default|GetFlipbook) "/Game/Assets/Player/WalkDown/FB_WalkDown.FB_WalkDown"))
    (:0
      (switch int (Math|Float|Truncate (.x _output_get))
        (:-1
          (Sprite|SetFlipbook (Variables|Default|GetFlipbook) "/Game/Assets/Player/WalkLeft/FB_WalkLeft.FB_WalkLeft"))
        (:1
          (Sprite|SetFlipbook (Variables|Default|GetFlipbook) "/Game/Assets/Player/WalkRight/FB_WalkRight.FB_WalkRight"))))
    (:1
      (Sprite|SetFlipbook (Variables|Default|GetFlipbook) "/Game/Assets/Player/WalkUp/FB_WalkUp.FB_WalkUp"))))

(event EventBeginPlay
  (Input|AddMappingContext (PlayerController|LocalPlayerSubsystems|GetEnhancedInputLocalPlayerSubsystem (Game|GetPlayerController 0)) "/Game/Input/IMC_Player.IMC_Player" 0 "(bIgnoreAllPressedKeysUntilRelease=True,bForceImmediately=False,bNotifyUserSettings=False)")
  (bind _returnvalue (UserInterface|CreateWidget "/Game/Widgets/W_Enemy.W_Enemy_C"))
  (UserInterface|SetWidget (Variables|Default|GetText) _returnvalue)
  (bind _returnvalue_2 (UserInterface|CreateWidget "/Game/Widgets/W_Toughts.W_Toughts_C"))
  (bind _output_get (Variables|Default|SetToughts _returnvalue_2))
  (UserInterface|Viewport|AddtoViewport _output_get 0))

(event Game|Damage|EventAnyDamage
  (params (Damage :type Float%20%28single-precision%29) (DamageType :type Damage%20Type%20Object%20Reference) (InstigatedBy :type Controller%20Object%20Reference) (DamageCauser :type Actor%20Object%20Reference))
  (bind _returnvalue (Game|GetPlayerController 0))
  (bind _flipbook (Variables|Default|GetFlipbook))
  ;[0.15 0.15 0.15 0.5] Decrease health from damage and show death menu if health<=0
  (Variables|Default|SetHealth (- (Variables|Default|GetHealth) Damage))
  (if (<= (Variables|Default|GetHealth) 0.0)
    (bind _returnvalue_2 (UserInterface|CreateWidget "/Game/Widgets/WB_DeathMenu.WB_DeathMenu_C"))
    (UserInterface|Viewport|AddtoViewport _returnvalue_2 0)
    (Variables|/Script/Engine.PlayerController|SetbShowMouseCursor _returnvalue true)
    (Input|SetInputModeUIOnly _returnvalue 0 "DoNotLock" false)
    (Game|SetGamePaused true)
    (else
      (Sprite|SetSpriteColor _flipbook "(R=0.293750,G=0.142591,B=0.142591,A=1.000000)")
      (Utilities|FlowControl|Delay 0.2)
      (Sprite|SetSpriteColor _flipbook "(R=1.000000,G=1.000000,B=1.000000,A=1.000000)"))))

(event EventTick
  (params (DeltaSeconds :type Float%20%28single-precision%29))
  (bind _returnvalue (Transformation|GetActorLocation))
  (bind _flipbook (Variables|Default|GetFlipbook))
  (CallFunction|DecreaseHunger (* DeltaSeconds 1.0))
  (if (not (Variables|Default|GetAttacking))
    (if (Utilities|Operators|EqualEqual :A (Variables|/Script/Engine.MovementComponent|GetVelocity (Variables|Default|GetFloatingPawnMovement)) :ErrorTolerance 0.1)
      (switch int (Math|Float|Truncate (Math|Float|Sign(Float) (.z (Variables|Default|GetDirection))))
        (:Default
          _)
        (:-1
          (Sprite|SetFlipbook _flipbook "/Game/Assets/Player/Idle/FB_PrisonerIdle.FB_PrisonerIdle" :!label _label))
        (:0
          (goto _label))
        (:1
          (Sprite|SetFlipbook _flipbook "/Game/Assets/Player/IdleUp/FB_IdleUp.FB_IdleUp"))))
    (bind _outhit (Collision|SphereTraceByChannel _returnvalue (+ _returnvalue (* (Variables|Default|GetDirection) "20.000000,0.000000,20.000000")) 4.0 "TraceTypeQuery3" false 0 "None"))
    (Class|BPIShowOptions|ShowOptions(Message) (.hitactor _outhit))))

(event Input|KeyboardEvents|Enter
  (params (Key :type Key%20Structure :default "None"))
  (:Pressed
    (Default|HideSelf (Variables|Default|GetToughts))))

(event Input|KeyboardEvents|SpaceBar
  (params (Key :type Key%20Structure :default "None"))
  (bind _returnvalue (Game|GetPlayerController 0))
  (bind _returnvalue_2 (Transformation|GetActorLocation))
  (bind _returnvalue_3 (Game|GetPlayerController 0))
  (bind _direction (Variables|Default|GetDirection))
  (bind _toughts (Variables|Default|GetToughts))
  (bind _flipbook (Variables|Default|GetFlipbook))
  (bind _toughts_2 (Variables|Default|GetToughts))
  (bind _text (Variables|/Game/Widgets/W_Toughts.W_Toughts_C|GetText _toughts_2))
  (:Pressed
    (if (not (Variables|Default|GetAttacking))
      (Variables|Default|SetAttacking true)
      (Input|DisableInput _returnvalue_3)
      (Audio|PlaySoundatLocation "/Game/Assets/Sound/punch.punch" (Transformation|GetActorLocation) "0, 0, 0" 1.0 1.0 0.0 0 0 0 0)
      (switch int (Math|Float|Truncate (Math|Float|Sign(Float) (.x _direction)))
        (:Default
          _)
        (:-1
          (Sprite|SetFlipbook (Variables|Default|GetFlipbook) "/Game/Assets/Player/AttackLeftRight/FB_AttackLeft.FB_AttackLeft"))
        (:0
          (switch int (Math|Float|Truncate (Math|Float|Sign(Float) (.z _direction)))
            (:Default
              _)
            (:-1
              (Sprite|SetFlipbook (Variables|Default|GetFlipbook) "/Game/Assets/Player/AttackDown/FB_AttackDown.FB_AttackDown"))
            (:0
              _)
            (:1
              (Sprite|SetFlipbook (Variables|Default|GetFlipbook) "/Game/Assets/Player/AttackUp/FB_AttackUp.FB_AttackUp"))))
        (:1
          (Sprite|SetFlipbook (Variables|Default|GetFlipbook) "/Game/Assets/Player/AttackLeftRight/FB_AttackRight.FB_AttackRight")))
      (Utilities|FlowControl|Delay 0.4)
      (Variables|Default|SetAttacking false)
      (Input|EnableInput _returnvalue_3)
      (bind _outhit (Collision|SphereTraceByChannel _returnvalue_2 (+ _returnvalue_2 (* (Variables|Default|GetDirection) "40.000000,0.000000,40.000000")) 4.0 "TraceTypeQuery3" false 0 "None"))
      (bind _asbp_rat (Utilities|Casting|CastToBP_Rat (.hitactor _outhit))
        (:then
          (if (> (Variables|/Game/Blueprints/BP_Rat.BP_Rat_C|GetHealth _asbp_rat) 0.0)
            (bind _output_get (Variables|/Game/Blueprints/BP_Rat.BP_Rat_C|SetHealth _asbp_rat (- (Variables|/Game/Blueprints/BP_Rat.BP_Rat_C|GetHealth _asbp_rat) (Variables|Default|GetDamage))))
            (Sprite|SetSpriteColor (Variables|/Game/Blueprints/BP_Rat.BP_Rat_C|GetPaperFlipbook _asbp_rat) "(R=0.582292,G=0.201983,B=0.201983,A=1.000000)")
            (Utilities|FlowControl|Delay 0.2)
            (Sprite|SetSpriteColor (Variables|/Game/Blueprints/BP_Rat.BP_Rat_C|GetPaperFlipbook _asbp_rat) "(R=1.000000,G=1.000000,B=1.000000,A=1.000000)")
            (if (<= _output_get 0.0)
              (if (Variables|Default|GetKilledRat)
                (Rendering|Components|TextRender|SetText _text "...another little one gone...")
                (else
                  (Variables|Default|SetKilledRat true)
                  (Rendering|Components|TextRender|SetText _text "...poor little guy...no matter, small price to pay for freedom...")))
              (Default|ShowSelf _toughts_2))))
        (:CastFailed
          (bind _asbp_guard_2 (Utilities|Casting|CastToBP_Guard2 (.hitactor _outhit))
            (:then
              (if (> (Variables|/Game/Blueprints/BP_Guard2.BP_Guard2_C|GetHealth _asbp_guard_2) 0.0)
                (bind _output_get_2 (Variables|/Game/Blueprints/BP_Guard2.BP_Guard2_C|SetHealth _asbp_guard_2 (- (Variables|/Game/Blueprints/BP_Guard2.BP_Guard2_C|GetHealth _asbp_guard_2) (Variables|Default|GetDamage))))
                (Sprite|SetSpriteColor (Variables|/Game/Blueprints/BP_Guard2.BP_Guard2_C|GetPaperFlipbook _asbp_guard_2) "(R=0.582292,G=0.201983,B=0.201983,A=1.000000)")
                (Utilities|FlowControl|Delay 0.2)
                (Sprite|SetSpriteColor (Variables|/Game/Blueprints/BP_Guard2.BP_Guard2_C|GetPaperFlipbook _asbp_guard_2) "(R=1.000000,G=1.000000,B=1.000000,A=1.000000)")
                (if (<= _output_get_2 0.0)
                  (Variables|Default|SetHunger 1e+02)
                  (Variables|Default|SetHealth 1e+02)
                  (Input|DisableInput _returnvalue)
                  (Variables|Default|SetAttacking true)
                  (Utilities|FlowControl|Delay 0.5)
                  (Input|DisableInput _returnvalue)
                  (bind _asw_enemy (Utilities|Casting|CastToW_Enemy (UserInterface|GetUserWidgetObject (Variables|Default|GetText))))
                  (Sprite|SetFlipbook _flipbook "/Game/Assets/Player/IdleUp/FB_IdleUp.FB_IdleUp")
                  (Utilities|FlowControl|Delay 1.5)
                  (Rendering|Components|TextRender|SetText (Variables|/Game/Widgets/W_Enemy.W_Enemy_C|GetEnemyText _asw_enemy) "...")
                  (Utilities|FlowControl|Delay 1.5)
                  (Sprite|SetFlipbook _flipbook "/Game/Assets/Player/Idle/FB_PrisonerIdle.FB_PrisonerIdle")
                  (Utilities|FlowControl|Delay 1.5)
                  (Rendering|Components|TextRender|SetText (Variables|/Game/Widgets/W_Enemy.W_Enemy_C|GetEnemyText _asw_enemy) "...is this it...?")
                  (Utilities|FlowControl|Delay 1.5)
                  (Sprite|SetFlipbook _flipbook "/Game/Assets/Player/IdleUp/FB_IdleUp.FB_IdleUp")
                  (Utilities|FlowControl|Delay 1.5)
                  (Rendering|Components|TextRender|SetText (Variables|/Game/Widgets/W_Enemy.W_Enemy_C|GetEnemyText _asw_enemy) "...")
                  (CameraFades|StartCameraFade :self (Variables|/Script/Engine.PlayerController|GetPlayerCameraManager (Game|GetPlayerController 0)) :ToAlpha 1.0 :Duration 2.0 :bShouldFadeAudio true :bHoldWhenFinished true))))
            (:CastFailed
              (bind _asbp_prisoner (Utilities|Casting|CastToBP_Prisoner (.hitactor _outhit)))
              (if (> (Variables|/Game/Blueprints/BP_Prisoner.BP_Prisoner_C|GetHealth _asbp_prisoner) 0.0)
                (bind _output_get_3 (Variables|/Game/Blueprints/BP_Prisoner.BP_Prisoner_C|SetHealth _asbp_prisoner (- (Variables|/Game/Blueprints/BP_Prisoner.BP_Prisoner_C|GetHealth _asbp_prisoner) (Variables|Default|GetDamage))))
                (Sprite|SetSpriteColor (Variables|/Game/Blueprints/BP_Prisoner.BP_Prisoner_C|GetPaperFlipbook _asbp_prisoner) "(R=0.582292,G=0.201983,B=0.201983,A=1.000000)")
                (Utilities|FlowControl|Delay 0.2)
                (Sprite|SetSpriteColor (Variables|/Game/Blueprints/BP_Prisoner.BP_Prisoner_C|GetPaperFlipbook _asbp_prisoner) "(R=1.000000,G=1.000000,B=1.000000,A=1.000000)")
                (if (<= _output_get_3 0.0)
                  (Variables|Default|SetKilledPrisoner true)
                  (Rendering|Components|TextRender|SetText (Variables|/Game/Widgets/W_Toughts.W_Toughts_C|GetText _toughts) "...my hands...took...a human's...life?...")
                  (Default|ShowSelf _toughts))))))))))

(event Input|KeyboardEvents|U
  (params (Key :type Key%20Structure :default "None"))
  (bind _returnvalue (Transformation|GetActorLocation))
  (:Pressed
    (bind _outhit (Collision|SphereTraceByChannel _returnvalue (+ _returnvalue (* (Variables|Default|GetDirection) "20.000000,0.000000,20.000000")) 4.0 "TraceTypeQuery3" false 0 "None"))
    (bind _asbp_door (Utilities|Casting|CastToBP_Door (.hitactor _outhit)))
    (if (Variables|/Game/Blueprints/BP_Door.BP_Door_C|GetLocked _asbp_door)
      (bind _asw_enemy (Utilities|Casting|CastToW_Enemy (UserInterface|GetUserWidgetObject (Variables|Default|GetText))))
      (if (Variables|Default|GetHasKey)
        (Audio|PlaySoundatLocation "/Game/Assets/Sound/lock-the-door-46014.lock-the-door-46014" (Transformation|GetActorLocation) "0, 0, 0" 1.0 1.0 0.0 0 0 0 0)
        (Variables|/Game/Blueprints/BP_Door.BP_Door_C|SetLocked _asbp_door false)
        (Variables|Default|SetHasKey false)
        (else
          (Rendering|Components|TextRender|SetText (Variables|/Game/Widgets/W_Enemy.W_Enemy_C|GetEnemyText _asw_enemy) "Need a key...")))
      (Utilities|FlowControl|Delay 2.0)
      (Rendering|Components|TextRender|SetText (Variables|/Game/Widgets/W_Enemy.W_Enemy_C|GetEnemyText _asw_enemy) ""))))

(event Input|KeyboardEvents|T
  (params (Key :type Key%20Structure :default "None"))
  (bind _returnvalue (Transformation|GetActorLocation))
  (:Pressed
    (bind _outhit (Collision|SphereTraceByChannel _returnvalue (+ _returnvalue (* (Variables|Default|GetDirection) "20.000000,0.000000,20.000000")) 4.0 "TraceTypeQuery3" false 0 "None"))
    (bind _asbp_food (Utilities|Casting|CastToBP_Food (.hitactor _outhit))
      (:then
        (Actor|DestroyActor _asbp_food)
        (Variables|Default|SetFood (+ (Variables|Default|GetFood) 1))
        (Audio|PlaySoundatLocation "/Game/Assets/Sound/bong_001.bong_001" (Transformation|GetActorLocation) "0, 0, 0" 1.0 1.0 0.0 0 0 0 0 :!label _label))
      (:CastFailed
        (bind _asbp_rat (Utilities|Casting|CastToBP_Rat (.hitactor _outhit)))
        (if (<= (Variables|/Game/Blueprints/BP_Rat.BP_Rat_C|GetHealth _asbp_rat) 0.0)
          (Actor|DestroyActor _asbp_rat)
          (Variables|Default|SetFood (+ (Variables|Default|GetFood) 1))
          (goto _label))))))

(event Input|KeyboardEvents|G
  (params (Key :type Key%20Structure :default "None"))
  (bind _returnvalue (Transformation|GetActorLocation))
  (:Pressed
    (bind _outhit (Collision|SphereTraceByChannel _returnvalue (+ _returnvalue (* (Variables|Default|GetDirection) "20.000000,0.000000,20.000000")) 4.0 "TraceTypeQuery3" false 0 "None"))
    (bind _asbp_prisoner (Utilities|Casting|CastToBP_Prisoner (.hitactor _outhit)))
    (if (>= (Variables|/Game/Blueprints/BP_Prisoner.BP_Prisoner_C|GetHunger _asbp_prisoner) 0)
      (if (> (Variables|Default|GetFood) 0)
        (if (Actor|ActorHasTag _asbp_prisoner "lead1")
          (bind _outactors (Actor|GetAllActorsOfClasswithTag "/Game/Blueprints/BP_Prisoner.BP_Prisoner_C" "lead2"))
          (for _array_element _outactors
            (if (< (Variables|/Game/Blueprints/BP_Prisoner.BP_Prisoner_C|GetHunger _array_element) 0)
              (Audio|PlaySoundatLocation "/Game/Assets/Sound/key-get-39925.key-get-39925" (Transformation|GetActorLocation) "0, 0, 0" 1.0 1.0 0.0 0 0 0 0)
              (Variables|/Game/Blueprints/BP_Prisoner.BP_Prisoner_C|SetHunger _asbp_prisoner -1)
              (Variables|Default|SetFood (- (Variables|Default|GetFood) 1))
              (Variables|Default|SetHasKey true)
              (else
                (Rendering|Components|TextRender|SetText (Variables|/Game/Widgets/W_Enemy.W_Enemy_C|GetEnemyText (stale Input|KeyboardEvents|U _asw_enemy)) "He is afraid they are gonna attack him...")
                (Utilities|FlowControl|Delay 2.0)
                (Rendering|Components|TextRender|SetText (Variables|/Game/Widgets/W_Enemy.W_Enemy_C|GetEnemyText (stale Input|KeyboardEvents|U _asw_enemy)) ""))))
          (else
            (if (Actor|ActorHasTag _asbp_prisoner "violent")
              (Audio|PlaySoundatLocation "/Game/Assets/Sound/key-get-39925.key-get-39925" (Transformation|GetActorLocation) "0, 0, 0" 1.0 1.0 0.0 0 0 0 0))
            (Variables|/Game/Blueprints/BP_Prisoner.BP_Prisoner_C|SetHunger _asbp_prisoner -1)
            (Variables|Default|SetFood (- (Variables|Default|GetFood) 1))
            (Variables|Default|SetHasKey true)))
        (else
          (bind _asw_enemy (Utilities|Casting|CastToW_Enemy (UserInterface|GetUserWidgetObject (Variables|Default|GetText))))
          (Rendering|Components|TextRender|SetText (Variables|/Game/Widgets/W_Enemy.W_Enemy_C|GetEnemyText _asw_enemy) "No food...")
          (Utilities|FlowControl|Delay 2.0)
          (Rendering|Components|TextRender|SetText (Variables|/Game/Widgets/W_Enemy.W_Enemy_C|GetEnemyText _asw_enemy) ""))))))

(event Input|KeyboardEvents|E
  (params (Key :type Key%20Structure :default "None"))
  (bind _returnvalue (Transformation|GetActorLocation))
  (bind _toughts (Variables|Default|GetToughts))
  (:Pressed
    (bind _outhit (Collision|SphereTraceByChannel _returnvalue (+ _returnvalue (* (Variables|Default|GetDirection) "20.000000,0.000000,20.000000")) 4.0 "TraceTypeQuery3" false 0 "None"))
    (bind _asbp_rat (Utilities|Casting|CastToBP_Rat (.hitactor _outhit)))
    (CallFunction|IncreaseHunger 2e+01)
    (Actor|DestroyActor _asbp_rat)
    (Variables|Default|SetAteRat true)
    (Rendering|Components|TextRender|SetText (Variables|/Game/Widgets/W_Toughts.W_Toughts_C|GetText _toughts) "...I...ate a rat?...the lengths we go to....")
    (Default|ShowSelf _toughts)))

(event Input|KeyboardEvents|O
  (params (Key :type Key%20Structure :default "None"))
  (bind _returnvalue (Transformation|GetActorLocation))
  (bind _direction (Variables|Default|GetDirection))
  (:Pressed
    (bind _outhit (Collision|SphereTraceByChannel _returnvalue (+ _returnvalue (* (Variables|Default|GetDirection) "20.000000,0.000000,20.000000")) 4.0 "TraceTypeQuery3" false 0 "None"))
    (bind _asbp_door (Utilities|Casting|CastToBP_Door (.hitactor _outhit)))
    (if (not (Variables|/Game/Blueprints/BP_Door.BP_Door_C|GetLocked _asbp_door))
      (if (== (* (.x _direction) (.z _direction)) 0.0)
        (Transformation|SetActorLocation (+ (* (Variables|Default|GetDirection) (+ (.distance _outhit) 1.1e+02)) (Transformation|GetActorLocation)) false false)
        (Class|BPIStageUnlocked|StageUnlocked(Message) _asbp_door)
        (Audio|PlaySoundatLocation "/Game/Assets/Sound/vault-2-100077.vault-2-100077" (Transformation|GetActorLocation) "0, 0, 0" 1.0 1.0 0.0 0 0 0 0)))))

(fn ConstructionScript)

(fn DealDamage
  (params (Enemy :type Actor%20Object%20Reference))
  (bind _asbp_rat (Utilities|Casting|CastToBP_Rat Enemy)
    (:then
      (Variables|/Game/Blueprints/BP_Rat.BP_Rat_C|SetHealth _asbp_rat (- (Variables|/Game/Blueprints/BP_Rat.BP_Rat_C|GetHealth _asbp_rat) (Variables|Default|GetDamage))))
    (:CastFailed
      (bind _asbp_guard_2 (Utilities|Casting|CastToBP_Guard2 Enemy)
        (:then
          (Variables|Default|SetHealth (- (Variables|/Game/Blueprints/BP_Guard2.BP_Guard2_C|GetHealth _asbp_guard_2) (Variables|Default|GetDamage))))
        (:CastFailed
          (bind _asbp_prisoner (Utilities|Casting|CastToBP_Prisoner Enemy))
          (Variables|/Game/Blueprints/BP_Prisoner.BP_Prisoner_C|SetHealth _asbp_prisoner (- (Variables|/Game/Blueprints/BP_Prisoner.BP_Prisoner_C|GetHealth _asbp_prisoner) (Variables|Default|GetDamage)))))))
  (Sprite|SetSpriteColor (Variables|/Game/Blueprints/BP_Rat.BP_Rat_C|GetPaperFlipbook _asbp_rat) "(R=0.582292,G=0.201983,B=0.201983,A=1.000000)"))