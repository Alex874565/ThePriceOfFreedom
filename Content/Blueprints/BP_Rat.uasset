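; BP_Rat is a rat actor that displays an eat-or-take prompt once it is dead and not yet eaten.
; It creates a W_Enemy widget on BeginPlay for its Text widget component, and the ShowOptions event writes the prompt when Health is depleted.
; A looping timer runs ResetText every second to clear the text once the player pawn is out of close range.
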(event EventBeginPlay
  (bind _returnvalue (UserInterface|CreateWidget "/Game/Widgets/W_Enemy.W_Enemy_C"))
  (UserInterface|SetWidget (Variables|Default|GetText) _returnvalue)
  (Utilities|Time|SetTimerbyFunctionName 0 "ResetText" 1.0 true))

(event Collision|EventActorBeginOverlap
  (params (OtherActor :type Actor%20Object%20Reference)))

(event EventTick
  (params (DeltaSeconds :type Float%20%28single-precision%29)))

(event EventShowOptions
  (bind _asw_enemy (Utilities|Casting|CastToW_Enemy (UserInterface|GetWidget (Variables|Default|GetText))))
  (if (<= (Variables|Default|GetHealth) 0.0)
    (if (not (Variables|Default|GetEaten))
      (Rendering|Components|TextRender|SetText (Variables|/Game/Widgets/W_Enemy.W_Enemy_C|GetEnemyText _asw_enemy) "(E) Eat 
(T) Take"))))

(fn ConstructionScript)

(fn ResetText
  (bind _asw_enemy (Utilities|Casting|CastToW_Enemy (UserInterface|GetUserWidgetObject (Variables|Default|GetText))))
  (if (>= (Transformation|GetDistanceTo (Game|Player|GetPlayerPawn 0)) 9e+01)
    (Rendering|Components|TextRender|SetText (Variables|/Game/Widgets/W_Enemy.W_Enemy_C|GetEnemyText _asw_enemy) "")))