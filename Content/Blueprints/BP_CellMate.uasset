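; BP_CellMate is a companion actor that keeps close to the player and displays a W_Enemy text widget.
; On BeginPlay it creates the widget, assigns it to its Text component and sets the text shadow to opaque white.
; While not Fighting, Tick snaps it to just behind the player on the X and Z axes, without sweep, whenever it falls too far away.
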(event EventBeginPlay
  (bind _returnvalue (UserInterface|CreateWidget "/Game/Widgets/W_Enemy.W_Enemy_C"))
  (UserInterface|SetWidget (Variables|Default|GetText) _returnvalue)
  (Variables|/Script/UMG.TextBlock|SetShadowColorAndOpacity (Variables|/Game/Widgets/W_Enemy.W_Enemy_C|GetEnemyText _returnvalue) "(R=1.000000,G=1.000000,B=1.000000,A=1.000000)"))

(event Collision|EventActorBeginOverlap
  (params (OtherActor :type Actor%20Object%20Reference)))

(event EventTick
  (params (DeltaSeconds :type Float%20%28single-precision%29))
  (bind _returnvalue (Game|Player|GetPlayerPawn 0))
  (bind _returnvalue_2 (Transformation|GetActorLocation))
  (bind _returnvalue_3 (Transformation|GetActorLocation _returnvalue))
  (bind _returnvalue_4 (- _returnvalue_3 _returnvalue_2))
  (if (not (Variables|Default|GetFighting))
    (if (>= (Transformation|GetDistanceTo _returnvalue) 1e+02)
      (Transformation|SetActorLocation (- _returnvalue_3 (Math|Vector|MakeVector (* (Math|Float|Sign(Float) (.x _returnvalue_4)) 2e+01) 0.0 (* (Math|Float|Sign(Float) (.z _returnvalue_4)) 2e+01))) false false))))

(fn ConstructionScript)