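; AI controller for the Paper2D rat enemy BP_Rat, which chases and melee-attacks the player.
; Tick shows a death flipbook at zero health, otherwise latches Attacking once the player overlaps the rat's sphere.
; An attacking rat moves straight at the player without pathfinding, flipping its sprite by X direction.
; At close range it halts and, after a delay guarded by Stopped, sphere-traces toward the player in X/Z to deal damage.
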(event EventBeginPlay
  (bind _asbp_rat (Utilities|Casting|CastToBP_Rat (Pawn|GetControlledPawn))))

(event EventTick
  (params (DeltaSeconds :type Float%20%28single-precision%29))
  (bind _returnvalue (Pawn|GetControlledPawn))
  (bind _returnvalue_2 (Game|Player|GetPlayerPawn 0))
  (bind _returnvalue_3 (Transformation|GetActorLocation _returnvalue))
  (bind _returnvalue_4 (Transformation|GetActorLocation _returnvalue_2))
  (bind _returnvalue_5 (- _returnvalue_4 _returnvalue_3))
  (bind _returnvalue_6 (Class|KismetMathLibrary|FMod64 (.x _returnvalue_5) 1e+01))
  (bind _returnvalue_7 (Class|KismetMathLibrary|SignOfInteger64 _returnvalue_6))
  (if (<= (Variables|/Game/Blueprints/BP_Rat.BP_Rat_C|GetHealth (stale EventBeginPlay _asbp_rat)) 0.0)
    (Sprite|SetFlipbook (Variables|/Game/Blueprints/BP_Rat.BP_Rat_C|GetPaperFlipbook (stale EventBeginPlay _asbp_rat)) "/Game/Assets/NPC/Rat/FB_Ratless.FB_Ratless")
    (elif (Variables|/Game/Blueprints/BP_Rat.BP_Rat_C|GetAttacking (stale EventBeginPlay _asbp_rat))
      (if (not (Variables|/Game/Blueprints/BP_Rat.BP_Rat_C|GetStopped (stale EventBeginPlay _asbp_rat)))
        (if (<= (Transformation|GetDistanceTo _returnvalue _returnvalue_2) 2e+01)
          (AI|Navigation|StopMovement)
          (Variables|/Game/Blueprints/BP_Rat.BP_Rat_C|SetStopped (stale EventBeginPlay _asbp_rat) true)
          (Sprite|SetFlipbook (Variables|/Game/Blueprints/BP_Rat.BP_Rat_C|GetPaperFlipbook (stale EventBeginPlay _asbp_rat)) "/Game/Assets/NPC/Rat/FB_Attack.FB_Attack")
          (Utilities|FlowControl|Delay 0.5)
          (if (not (<= (Variables|/Game/Blueprints/BP_Rat.BP_Rat_C|GetHealth (stale EventBeginPlay _asbp_rat)) 0.0))
            (bind _outhit (Collision|SphereTraceByChannel _returnvalue_3 (+ _returnvalue_3 (Math|Vector|MakeVector (* _returnvalue_7 5.0) 0.0 (* (Class|KismetMathLibrary|SignOfInteger64 (.ReturnValue (Class|KismetMathLibrary|FMod64 (.z _returnvalue_5) 1e+01))) 5.0))) 1e+01 "TraceTypeQuery4" false 0 "None"))
            (Sprite|SetFlipbook (Variables|/Game/Blueprints/BP_Rat.BP_Rat_C|GetPaperFlipbook (stale EventBeginPlay _asbp_rat)) "/Game/Assets/NPC/Rat/FB_Idle.FB_Idle")
            (Variables|/Game/Blueprints/BP_Rat.BP_Rat_C|SetStopped (stale EventBeginPlay _asbp_rat) false)
            (bind _asbp_player (Utilities|Casting|CastToBP_Player (.hitactor _outhit)))
            (Game|Damage|ApplyDamage _asbp_player 1e+01 0 0)
            (Audio|PlaySound2D "/Game/Assets/Sound/man_hurt3.man_hurt3" 1.0 1.0 0.0 0 0))
          (else
            (AI|Navigation|MovetoLocation _returnvalue_4 0.0 false false false true 0)
            (if (< _returnvalue_7 0)
              (Transformation|SetRelativeRotation (Variables|/Game/Blueprints/BP_Rat.BP_Rat_C|GetPaperFlipbook (stale EventBeginPlay _asbp_rat)) "0, 0, 0" false false)
              (else
                (Transformation|SetRelativeRotation (Variables|/Game/Blueprints/BP_Rat.BP_Rat_C|GetPaperFlipbook (stale EventBeginPlay _asbp_rat)) "0.000000,180.000000,0.000000" false false))))))
      (else
        (bind _playerclose (CallFunction|CheckPlayerClose (stale EventBeginPlay _asbp_rat)))
        (if _playerclose
          (Variables|/Game/Blueprints/BP_Rat.BP_Rat_C|SetAttacking (stale EventBeginPlay _asbp_rat) true))))))

(fn ConstructionScript)

(fn CheckPlayerClose
  (params (Actor :type BP%20Rat%20Object%20Reference))
  (return (Collision|IsOverlappingActor (Variables|/Game/Blueprints/BP_Rat.BP_Rat_C|GetSphere Actor) (Game|Player|GetPlayerPawn 0) :!class /Script/Engine.PrimitiveComponent)))