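; BP_Prisoner is a 2D flipbook prisoner NPC with a floating text widget that can offer a give-food option.
; Tick switches to the idle flipbook while it is alive and stationary.
; ShowOptions appends the "(G) Give Food" prompt once if health and hunger checks pass.
; A looping timer runs ResetText, trimming the text back to TextLength when the player is out of range.
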(event EventBeginPlay
  (bind _returnvalue (UserInterface|CreateWidget "/Game/Widgets/W_Enemy.W_Enemy_C"))
  (UserInterface|SetWidget (Variables|Default|GetText) _returnvalue)
  (Utilities|Time|SetTimerbyFunctionName 0 "ResetText" 1.0 true))

(event Collision|EventActorBeginOverlap
  (params (OtherActor :type Actor%20Object%20Reference)))

(event EventTick
  (params (DeltaSeconds :type Float%20%28single-precision%29))
  (if (and (Utilities|Operators|EqualEqual :A (Variables|/Script/Engine.MovementComponent|GetVelocity (Variables|Default|GetFloatingPawnMovement)) :ErrorTolerance 0.1) (> (Variables|Default|GetHealth) 0.0))
    (Sprite|SetFlipbook (Variables|Default|GetPaperFlipbook) "/Game/Assets/Player/Idle/FB_PrisonerIdle.FB_PrisonerIdle")))

(event EventShowOptions
  (bind _asw_enemy (Utilities|Casting|CastToW_Enemy (UserInterface|GetWidget (Variables|Default|GetText))))
  (if (and (> (Variables|Default|GetHealth) 0.0) (>= (Variables|Default|GetHunger) 0))
    (if (not (Utilities|String|Contains (Utilities|String|ToString(Text) (Class|TextBlock|GetText (Variables|/Game/Widgets/W_Enemy.W_Enemy_C|GetEnemyText _asw_enemy))) "Give Food"))
      (Rendering|Components|TextRender|SetText (Variables|/Game/Widgets/W_Enemy.W_Enemy_C|GetEnemyText _asw_enemy) (Utilities|Text|ToText(String) (Utilities|String|Append (Utilities|String|ToString(Text) (Class|TextBlock|GetText (Variables|/Game/Widgets/W_Enemy.W_Enemy_C|GetEnemyText _asw_enemy))) " 
(G) Give Food"))))))

(fn ConstructionScript)

(fn ResetText
  (bind _asw_enemy (Utilities|Casting|CastToW_Enemy (UserInterface|GetUserWidgetObject (Variables|Default|GetText))))
  (if (>= (Transformation|GetDistanceTo (Game|Player|GetPlayerPawn 0)) 9e+01)
    (Rendering|Components|TextRender|SetText (Variables|/Game/Widgets/W_Enemy.W_Enemy_C|GetEnemyText _asw_enemy) (Utilities|Text|ToText(String) (Utilities|String|GetSubstring (Utilities|String|ToString(Text) (Class|TextBlock|GetText (Variables|/Game/Widgets/W_Enemy.W_Enemy_C|GetEnemyText _asw_enemy))) 0 (Variables|Default|GetTextLength))))))