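; AI controller for the cellmate buddy, a Paper2D companion that trails the player.
; On BeginPlay it caches the pawn and, after a short delay, shows a greeting in the pawn's text widget.
; Each tick, unless the mate is dead or fighting, it moves straight at the player without pathfinding.
; Flipbooks show idle on arrival, otherwise up/down from the Z offset, falling back to left/right from X when the Z offset is small.
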(event EventBeginPlay
  (bind _asbp_cell_mate (Utilities|Casting|CastToBP_CellMate (Pawn|GetControlledPawn)))
  (Utilities|FlowControl|Delay 1.0)
  (bind _asw_enemy (Utilities|Casting|CastToW_Enemy (UserInterface|GetUserWidgetObject (Variables|/Game/Blueprints/BP_CellMate.BP_CellMate_C|GetText _asbp_cell_mate))))
  (Rendering|Components|TextRender|SetText (Variables|/Game/Widgets/W_Enemy.W_Enemy_C|GetEnemyText _asw_enemy) "BUDDY 
Mornin', friend! We finally got the key! Let's go!"))

(event EventTick
  (params (DeltaSeconds :type Float%20%28single-precision%29))
  (bind _returnvalue (Pawn|GetControlledPawn))
  (bind _returnvalue_2 (Game|Player|GetPlayerPawn 0))
  (bind _returnvalue_3 (Transformation|GetActorLocation _returnvalue_2))
  (bind _returnvalue_4 (Transformation|GetActorLocation _returnvalue))
  (bind _returnvalue_5 (- _returnvalue_3 _returnvalue_4))
  (if (not (Variables|/Game/Blueprints/BP_CellMate.BP_CellMate_C|GetDead (stale EventBeginPlay _asbp_cell_mate)))
    (if (not (Variables|/Game/Blueprints/BP_CellMate.BP_CellMate_C|GetFighting (stale EventBeginPlay _asbp_cell_mate)))
      (bind _returnvalue_6 (AI|Navigation|MovetoLocation _returnvalue_3 4.0 true false false true 0))
      (if (Utilities|Enum|Equal(Enum) _returnvalue_6 "AlreadyAtGoal")
        (Sprite|SetFlipbook (Variables|/Game/Blueprints/BP_CellMate.BP_CellMate_C|GetPaperFlipbook (stale EventBeginPlay _asbp_cell_mate)) "/Game/Assets/NPC/Mate/Idle/FB_MateIdle.FB_MateIdle")
        (else
          (switch int (Math|Float|Truncate (Math|Float|Sign(Float) (Math|Conversions|ToFloat(Integer) (.ReturnValue (Math|Float|Division(WholeandRemainder) (.z _returnvalue_5) 1e+01)))))
            (:-1
              (Sprite|SetFlipbook (Variables|/Game/Blueprints/BP_CellMate.BP_CellMate_C|GetPaperFlipbook (stale EventBeginPlay _asbp_cell_mate)) "/Game/Assets/NPC/Mate/MoveDown/FB_MateDown.FB_MateDown"))
            (:0
              (switch int (Math|Float|Truncate (Math|Float|Sign(Float) (.x _returnvalue_5)))
                (:-1
                  (Sprite|SetFlipbook (Variables|/Game/Blueprints/BP_CellMate.BP_CellMate_C|GetPaperFlipbook (stale EventBeginPlay _asbp_cell_mate)) "/Game/Assets/NPC/Mate/MoveLeft/FB_MateLeft.FB_MateLeft"))
                (:1
                  (Sprite|SetFlipbook (Variables|/Game/Blueprints/BP_CellMate.BP_CellMate_C|GetPaperFlipbook (stale EventBeginPlay _asbp_cell_mate)) "/Game/Assets/NPC/Mate/MoveRight/FB_MateRight.FB_MateRight"))))
            (:1
              (Sprite|SetFlipbook (Variables|/Game/Blueprints/BP_CellMate.BP_CellMate_C|GetPaperFlipbook (stale EventBeginPlay _asbp_cell_mate)) "/Game/Assets/NPC/Mate/MoveUp/FB_MateUp.FB_MateUp"))))))))

(fn ConstructionScript)