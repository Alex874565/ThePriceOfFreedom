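; BP_Guard is a flipbook guard that starts a scripted escape scene when the player comes within range.
; Tick polls distance, then once disables player input, shows a shout on its W_Enemy widget, plays a yell and sets the player's HUD to "RUN!!!".
; It then uses Delays to script BP_CellMate's dialogue and move to FightLocation, switches both to fight flipbooks with sound, and restores input.
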(event EventBeginPlay
  (bind _returnvalue (UserInterface|CreateWidget "/Game/Widgets/W_Enemy.W_Enemy_C"))
  (UserInterface|SetWidget (Variables|Default|GetText) _returnvalue))

(event Collision|EventActorBeginOverlap
  (params (OtherActor :type Actor%20Object%20Reference)))

(event EventTick
  (params (DeltaSeconds :type Float%20%28single-precision%29))
  (bind _returnvalue (Game|GetPlayerController 0))
  (bind _returnvalue_2 (Game|Player|GetPlayerPawn 0))
  (if (not (Variables|Default|GetDead))
    (if (and (< (Transformation|GetDistanceTo (Game|Player|GetPlayerPawn 0)) 5e+01) (not (Variables|Default|GetAlert)))
      (Variables|Default|SetAlert true)
      (Input|DisableInput _returnvalue_2 _returnvalue)
      (Rendering|Components|TextRender|SetText (Variables|/Game/Widgets/W_Enemy.W_Enemy_C|GetEnemyText (stale EventBeginPlay _returnvalue)) "HEY, YOU! STOP RIGHT THERE!")
      (Audio|PlaySoundatLocation "/Game/Assets/Sound/guard_yell_hey.guard_yell_hey" (Transformation|GetActorLocation) "0, 0, 0" 1.0 1.0 0.0 0 0 0 0)
      (bind _asbp_player (Utilities|Casting|CastToBP_Player _returnvalue_2))
      (Rendering|Components|TextRender|SetText (Variables|/Game/Widgets/WB_HUD.WB_HUD_C|GetMissionText (Variables|/Game/Blueprints/BP_Player.BP_Player_C|GetHUD _asbp_player)) "RUN!!!")
      (bind _outactors (Actor|GetAllActorsOfClass "/Game/Blueprints/BP_CellMate.BP_CellMate_C"))
      (for _array_element _outactors
        (bind _asw_enemy (Utilities|Casting|CastToW_Enemy (UserInterface|GetUserWidgetObject (Variables|/Game/Blueprints/BP_CellMate.BP_CellMate_C|GetText _array_element))))
        (Utilities|FlowControl|Delay 1.5)
        (Rendering|Components|TextRender|SetText (Variables|/Game/Widgets/W_Enemy.W_Enemy_C|GetEnemyText _asw_enemy) "I'll stall him! Grab the key and GO!!")
        (Variables|/Game/Blueprints/BP_CellMate.BP_CellMate_C|SetFighting _array_element true)
        (Utilities|FlowControl|Delay 1.5)
        (switch int (Math|Float|Truncate (Math|Float|Sign(Float) (.z (- (Variables|/Game/Blueprints/BP_CellMate.BP_CellMate_C|GetFightLocation _array_element) (Transformation|GetActorLocation _array_element)))))
          (:-1
            (Sprite|SetFlipbook (Variables|/Game/Blueprints/BP_CellMate.BP_CellMate_C|GetPaperFlipbook _array_element) "/Game/Assets/NPC/Mate/MoveDown/FB_MateDown.FB_MateDown"))
          (:1
            (Sprite|SetFlipbook (Variables|/Game/Blueprints/BP_CellMate.BP_CellMate_C|GetPaperFlipbook _array_element) "/Game/Assets/NPC/Mate/MoveUp/FB_MateUp.FB_MateUp")))
        (AI|Navigation|MovetoLocation (AI|GetAIController _array_element) (Variables|/Game/Blueprints/BP_CellMate.BP_CellMate_C|GetFightLocation _array_element) 0.0 false false false true 0)
        (Utilities|FlowControl|Delay 1.25)
        (Audio|PlaySoundatLocation "/Game/Assets/Sound/Fight_Scene_with_Two_Men_Fighting_with_Punches__Grunts___Crashes.Fight_Scene_with_Two_Men_Fighting_with_Punches__Grunts___Crashes" (Transformation|GetActorLocation) "0, 0, 0" 1.0 1.0 0.0 "/Game/Assets/Sound/NewSoundAttenuation.NewSoundAttenuation" 0 0 0)
        (Rendering|Components|TextRender|SetText (Variables|/Game/Widgets/W_Enemy.W_Enemy_C|GetEnemyText _asw_enemy) "%$@#@")
        (Rendering|Components|TextRender|SetText (Variables|/Game/Widgets/W_Enemy.W_Enemy_C|GetEnemyText (stale EventBeginPlay _returnvalue)) "#@!#$!@")
        (Sprite|SetFlipbook (Variables|/Game/Blueprints/BP_CellMate.BP_CellMate_C|GetPaperFlipbook _array_element) "/Game/Assets/NPC/Mate/Fight/FB_MateFight.FB_MateFight")
        (Sprite|SetFlipbook (Variables|Default|GetPaperFlipbook) "/Game/Assets/NPC/Guard/Fight/FB_GuardFight.FB_GuardFight")
        (Input|EnableInput _returnvalue_2 _returnvalue)))))

(fn ConstructionScript)