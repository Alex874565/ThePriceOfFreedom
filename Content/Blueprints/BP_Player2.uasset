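; BP_Player2 is a player-named actor that plays a scripted ending cutscene through an on-screen dialogue widget.
; On BeginPlay it creates a W_Enemy widget and assigns it to its Text widget component.
; StartCutscene steps through timed lines of speech on that widget, then fades the camera and audio to black and opens the main menu map.
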(event EventBeginPlay
  (bind _returnvalue (UserInterface|CreateWidget "/Game/Widgets/W_Enemy.W_Enemy_C"))
  (UserInterface|SetWidget (Variables|Default|GetText) _returnvalue))

(event Collision|EventActorBeginOverlap
  (params (OtherActor :type Actor%20Object%20Reference)))

(event EventTick
  (params (DeltaSeconds :type Float%20%28single-precision%29)))

(event EventStartCutscene
  (Rendering|Components|TextRender|SetText (Variables|/Game/Widgets/W_Enemy.W_Enemy_C|GetEnemyText (stale EventBeginPlay _returnvalue)) "Finally!!!")
  (Utilities|FlowControl|Delay 3.0)
  (Rendering|Components|TextRender|SetText (Variables|/Game/Widgets/W_Enemy.W_Enemy_C|GetEnemyText (stale EventBeginPlay _returnvalue)) "Freedom!!!")
  (Utilities|FlowControl|Delay 3.0)
  (Rendering|Components|TextRender|SetText (Variables|/Game/Widgets/W_Enemy.W_Enemy_C|GetEnemyText (stale EventBeginPlay _returnvalue)) "...")
  (Utilities|FlowControl|Delay 3.0)
  (Rendering|Components|TextRender|SetText (Variables|/Game/Widgets/W_Enemy.W_Enemy_C|GetEnemyText (stale EventBeginPlay _returnvalue)) "...what have I done...")
  (Utilities|FlowControl|Delay 3.0)
  (Rendering|Components|TextRender|SetText (Variables|/Game/Widgets/W_Enemy.W_Enemy_C|GetEnemyText (stale EventBeginPlay _returnvalue)) "")
  (CameraFades|StartCameraFade :self (Variables|/Script/Engine.PlayerController|GetPlayerCameraManager (Game|GetPlayerController 0)) :ToAlpha 1.0 :Duration 2.0 :bShouldFadeAudio true :bHoldWhenFinished true)
  (Utilities|FlowControl|Delay 3.0)
  (Game|OpenLevel(byObjectReference) "/Game/Levels/MainMenuMap.MainMenuMap"))

(fn ConstructionScript)