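; BP_Guard2 is a guard character that shows a flipbook sprite and floating dialogue reacting to its Health.
; BeginPlay creates a W_Enemy widget on its Text component and sets an opening warning line.
; Every Tick, a chain of Health thresholds swaps the flipbook to increasingly bloodied and finally dead sprites, while the text shifts from warnings to pleas, clearing on death.
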(event EventBeginPlay
  (bind _returnvalue (UserInterface|CreateWidget "/Game/Widgets/W_Enemy.W_Enemy_C"))
  (UserInterface|SetWidget (Variables|Default|GetText) _returnvalue)
  (Rendering|Components|TextRender|SetText (Variables|/Game/Widgets/W_Enemy.W_Enemy_C|GetEnemyText _returnvalue) "Hey, you aren't allowed here!"))

(event Collision|EventActorBeginOverlap
  (params (OtherActor :type Actor%20Object%20Reference)))

(event EventTick
  (params (DeltaSeconds :type Float%20%28single-precision%29))
  (bind _paperflipbook (Variables|Default|GetPaperFlipbook))
  (if (<= (Variables|Default|GetHealth) 175.0)
    (if (<= (Variables|Default|GetHealth) 125.0)
      (if (<= (Variables|Default|GetHealth) 75.0)
        (if (<= (Variables|Default|GetHealth) 2e+01)
          (if (<= (Variables|Default|GetHealth) 0.0)
            (Sprite|SetFlipbook _paperflipbook "/Game/Assets/NPC/Guard/Death/FB_GuardDead.FB_GuardDead")
            (Rendering|Components|TextRender|SetText (Variables|/Game/Widgets/W_Enemy.W_Enemy_C|GetEnemyText (stale EventBeginPlay _returnvalue)) "")
            (else
              (Sprite|SetFlipbook _paperflipbook "/Game/Assets/NPC/Guard2/FB_BloodGuard2.FB_BloodGuard2")
              (Rendering|Components|TextRender|SetText (Variables|/Game/Widgets/W_Enemy.W_Enemy_C|GetEnemyText (stale EventBeginPlay _returnvalue)) "At least I die with a clean conscience...")))
          (else
            (Sprite|SetFlipbook _paperflipbook "/Game/Assets/NPC/Guard2/FB_BloodGuard.FB_BloodGuard")
            (Rendering|Components|TextRender|SetText (Variables|/Game/Widgets/W_Enemy.W_Enemy_C|GetEnemyText (stale EventBeginPlay _returnvalue)) "Please... I have a family...")))
        (else
          (Sprite|SetFlipbook _paperflipbook "/Game/Assets/NPC/Guard2/FB_BloodGuard.FB_BloodGuard")
          (Rendering|Components|TextRender|SetText (Variables|/Game/Widgets/W_Enemy.W_Enemy_C|GetEnemyText (stale EventBeginPlay _returnvalue)) "Stop! It hurts!")))
      (else
        (Sprite|SetFlipbook _paperflipbook "/Game/Assets/NPC/Guard2/FB_BloodlessGuard1.FB_BloodlessGuard1")
        (Rendering|Components|TextRender|SetText (Variables|/Game/Widgets/W_Enemy.W_Enemy_C|GetEnemyText (stale EventBeginPlay _returnvalue)) "Leave! I don't wanna fight you...")))))

(fn ConstructionScript)